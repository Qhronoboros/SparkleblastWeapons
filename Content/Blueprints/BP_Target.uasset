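; BP_Target is a damageable target actor that flashes when hit and destroys itself on death.
; It reacts to events from a BPC_Health component.
; The construction script makes a dynamic material instance on the sphere and caches its base color.
; Damage sets that color to a hit color, then restores it after a short delay, with a flag blocking overlapping flashes.
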(event `self.BPC_Health.OnDamage`
  (if (not (`self.VisualHitOnCooldown`))
    (`MaterialInstanceDynamic.SetVectorParameterValue` (`self.Material`) "Base Color" (`self.HitColor`))
    (set `self.VisualHitOnCooldown` true)
    (`KismetSystemLibrary.Delay` 0.1)
    (`MaterialInstanceDynamic.SetVectorParameterValue` (`self.Material`) "Base Color" (`self.DefaultColor`))
    (set `self.VisualHitOnCooldown` false)))

(event `self.BPC_Health.OnDeath`
  (`self.K2_DestroyActor`))

(fn `UserConstructionScript`
  (bind _sphere (`self.Sphere`))
  (bind _returnvalue (`PrimitiveComponent.CreateDynamicMaterialInstance` _sphere 0 (`PrimitiveComponent.GetMaterial` _sphere 0) "None"))
  (bind _output_get (set `self.Material` _returnvalue))
  (bind _returnvalue_2 (`MaterialInstanceDynamic.K2_GetVectorParameterValue` _output_get "Base Color"))
  (set `self.DefaultColor` _returnvalue_2))