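; Blueprint function library that gives the game a shared interface to FMOD audio.
; Bank helpers load or unload after checking loaded state, while one-shot helpers validate the event, auto-load its bank, then play it in 2D, at a location or attached.
; An FMOD subsystem handles event instances, global instances and the single music instance behind the music controls.
; PauseGameAudio and ResumeGameAudio are no-ops, with their bus-pause calls left unconnected.
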(fn `AutoLoadBank`
  (params (Event :type "FMODEvent Object Reference"))
  (`FMODSubsystem.AutoLoadBank` (subsystem `FMODSubsystem`) Event))

(fn `ChangeMusic`
  (params (NewEventInstance :type "FMODEventInstance Structure"))
  (bind _music_instance (`self.GetMusicInstance` (`local.__WorldContext`)))
  (`self.StopEventInstance` _music_instance true (`local.__WorldContext`))
  (bind _result (`self.SetMusicInstance` (`local.NewEventInstance`) (`local.__WorldContext`)))
  (if (not _result)
    (`KismetSystemLibrary.PrintString` (`local.__WorldContext`) "Could not set Music Instance, given Event Instance was invalid" true true (struct :`R` 1.0 :`A` 1.0))))

(fn `CheckEventInstancePlaybackState`
  (params (EventInstance :type "FMODEventInstance Structure") (Starting :type Boolean) (Playing :type Boolean) (Stopping :type Boolean) (Stopped :type Boolean))
  (returns (Result :type Boolean))
  (bind _returnvalue (`FMODSubsystem.GetPlaybackState` (subsystem `FMODSubsystem`) EventInstance))
  (if (!= _returnvalue 5)
    (return (select `int` _returnvalue :`0` (`local.Playing`) :`1` false :`2` (`local.Stopped`) :`3` (`local.Starting`) :`4` (`local.Stopping`)))
    (else
      (return false))))

(fn `CheckIsEventInstanceValid`
  (params (EventInstance :type "FMODEvent Object Reference"))
  (returns (Result :type Boolean))
  (return (`KismetSystemLibrary.IsValid` EventInstance)))

(fn `CreateEventInstance`
  (params (Event :type "FMODEvent Object Reference"))
  (returns (EventInstance :type "FMODEventInstance Structure"))
  (bind _returnvalue (`FMODSubsystem.CreateEventInstance` (subsystem `FMODSubsystem`) Event))
  (return _returnvalue))

(fn `CreateInstanceAttached`
  (params (Event :type "FMODEvent Object Reference") (AttachComponent :type "SceneComponent Object Reference") (StopPlayingIfDestroyed :type Boolean))
  (returns (AudioComponent :type "FMODAudioComponent Object Reference"))
  (`self.AutoLoadBank` Event (`local.__WorldContext`))
  (bind _returnvalue (`FMODBlueprintStatics.PlayEventAttached` Event (`local.AttachComponent`) "None" (0.0 0.0 0.0) "KeepRelativeOffset" (`local.StopPlayingIfDestroyed`) false false))
  (return _returnvalue))

(fn `GetGlobalEventInstance`
  (params (Event :type "FMODEvent Object Reference") (CreateNewIfEmpty :type Boolean))
  (returns (EventInstance :type "FMODEventInstance Structure"))
  (return (`FMODSubsystem.GetGlobalEventInstance` (subsystem `FMODSubsystem`) Event CreateNewIfEmpty)))

(fn `GetMusicInstance`
  (returns (`Music Instance` :type "FMODEventInstance Structure"))
  (bind _musicinstance (`FMODSubsystem.MusicInstance` (subsystem `FMODSubsystem`)))
  (bind _returnvalue (`FMODBlueprintStatics.EventInstanceIsValid` _musicinstance))
  (if _returnvalue
    (return _musicinstance)
    (else
      (`KismetSystemLibrary.PrintString` (`local.__WorldContext`) "MusicInstance is invalid" true true (struct :`R` 1.0 :`G` 0.040276 :`A` 1.0)))))

(fn `LoadBank`
  (params (Bank :type "FMODBank Object Reference"))
  (bind _returnvalue (`FMODBlueprintStatics.IsBankLoaded` Bank))
  (if (not _returnvalue)
    (`FMODBlueprintStatics.LoadBank` (`local.Bank`) true true)))

(fn `LoadBanks`
  (params (Banks :type "Set of FMODBank Object Reference"))
  (bind _valuepin (`|SetForEach` Banks)
    (:`then`
      (`self.LoadBank` _valuepin (`local.__WorldContext`)))))

(fn `PauseGameAudio`)

(fn `PauseMusic`
  (bind _music_instance (`self.GetMusicInstance` (`local.__WorldContext`)))
  (`FMODBlueprintStatics.EventInstanceSetPaused` _music_instance true))

(fn `PlayEventInstance`
  (params (EventInstance :type "FMODEventInstance Structure"))
  (returns (Result :type Boolean))
  (bind _returnvalue (`FMODSubsystem.PlayEventInstance` (subsystem `FMODSubsystem`) EventInstance))
  (return _returnvalue))

(fn `PlayMusic`
  (bind _music_instance (`self.GetMusicInstance` (`local.__WorldContext`)))
  (`self.ResumeMusic` (`local.__WorldContext`))
  (bind _result (`self.PlayEventInstance` _music_instance (`local.__WorldContext`)))
  (if (not _result)
    (`KismetSystemLibrary.PrintString` (`local.__WorldContext`) "Music could not be played" true true (struct :`R` 1.0 :`A` 1.0))))

(fn `PlayOneShot2D`
  (params (Event :type "FMODEvent Object Reference"))
  (if (`self.CheckIsEventInstanceValid` Event (`local.__WorldContext`))
    (`self.AutoLoadBank` (`local.Event`) (`local.__WorldContext`))
    (bind _returnvalue (`FMODBlueprintStatics.PlayEvent2D` (`local.Event`)))
    (`FMODBlueprintStatics.EventInstanceRelease` _returnvalue)))

(fn `PlayOneShotAtLocation`
  (params (Event :type "FMODEvent Object Reference") (Location :type "Vector Structure"))
  (if (`self.CheckIsEventInstanceValid` Event (`local.__WorldContext`))
    (`self.AutoLoadBank` (`local.Event`) (`local.__WorldContext`))
    (bind _returnvalue (`FMODBlueprintStatics.PlayEventAtLocation` (`local.Event`) (`KismetMathLibrary.Conv_VectorToTransform` (`local.Location`))))
    (`FMODBlueprintStatics.EventInstanceRelease` _returnvalue)))

(fn `PlayOneShotAttached`
  (params (Event :type "FMODEvent Object Reference") (AttachComponent :type "SceneComponent Object Reference") (StopPlayingIfDestroyed :type Boolean))
  (if (`self.CheckIsEventInstanceValid` Event (`local.__WorldContext`))
    (`self.AutoLoadBank` (`local.Event`) (`local.__WorldContext`))
    (`FMODBlueprintStatics.PlayEventAttached` (`local.Event`) (`local.AttachComponent`) "None" (0.0 0.0 0.0) "KeepRelativeOffset" (`local.StopPlayingIfDestroyed`))))

(fn `RemoveGlobalEventInstance`
  (params (EventInstance :type "FMODEventInstance Structure"))
  (returns (RemovedInstance :type Boolean))
  (bind _returnvalue (`FMODSubsystem.RemoveGlobalEventInstance` (subsystem `FMODSubsystem`) EventInstance))
  (return _returnvalue))

(fn `ResumeGameAudio`)

(fn `ResumeMusic`
  (bind _music_instance (`self.GetMusicInstance` (`local.__WorldContext`)))
  (`FMODBlueprintStatics.EventInstanceSetPaused` _music_instance))

(fn `SetGlobalEventInstance`
  (params (EventInstance :type "FMODEventInstance Structure") (ShouldReplace :type Boolean))
  (`FMODSubsystem.SetGlobalEventInstance` (subsystem `FMODSubsystem`) EventInstance ShouldReplace))

(fn `SetMusicInstance`
  (params (NewMusicInstance :type "FMODEventInstance Structure"))
  (returns (Result :type Boolean))
  (bind _returnvalue (`FMODSubsystem.SetMusicInstance` (subsystem `FMODSubsystem`) NewMusicInstance))
  (return _returnvalue))

(fn `StopEventInstance`
  (params (EventInstance :type "FMODEventInstance Structure") (Release :type Boolean))
  (`FMODBlueprintStatics.EventInstanceStop` EventInstance Release))

(fn `StopMusic`
  (bind _music_instance (`self.GetMusicInstance` (`local.__WorldContext`)))
  (`self.StopEventInstance` _music_instance false (`local.__WorldContext`)))

(fn `UnloadBank`
  (params (Bank :type "FMODBank Object Reference"))
  (bind _returnvalue (`FMODBlueprintStatics.IsBankLoaded` Bank))
  (if _returnvalue
    (`FMODBlueprintStatics.UnloadBank` Bank)))

(fn `UnloadBanks`
  (params (Banks :type "Set of FMODBank Object Reference"))
  (bind _valuepin (`|SetForEach` Banks)
    (:`then`
      (`self.UnloadBank` _valuepin (`local.__WorldContext`)))))

(fn `UpdateLoadedBanks`
  (params (NewBanks :type "Set of FMODBank Object Reference"))
  (`FMODSubsystem.UpdateLoadedBanks` (subsystem `FMODSubsystem`) NewBanks))