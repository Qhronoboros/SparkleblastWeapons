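; Component that picks a projectile's start location and direction according to a shoot origin mode: Owner, Muzzle, or Muzzle Owner.
; GetBulletOrigin randomizes the chosen owner or muzzle direction within a spread cone, then passes it to a per-mode GetVectors helper.
; Muzzle Owner mode combines the muzzle location with the owner's direction, and also feeds the owner location to its helper.
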(fn `GetBulletOrigin`
  (params (ShootOrigin :type "/Game/Blueprints/Guns/E_ShootOrigin Enum" :default "NewEnumerator0") (Spread :type "Float (double-precision)") (OwnerLocation :type "Vector Structure") (OwnerDirection :type "Vector Structure") (MuzzleLocation :type "Vector Structure") (MuzzleDirection :type "Vector Structure"))
  (returns (StartLocation :type "Vector Structure") (Direction :type "Vector Structure"))
  (bind (_outstartposition _outdirection) (`self.GetVectorsOwner` (`local.OwnerLocation`) (`self.GetRandomDirection` (`local.OwnerDirection`) (`local.Spread`))))
  (bind (_outstartposition_2 _outdirection_2) (`self.GetVectorsMuzzle` (`local.MuzzleLocation`) (`self.GetRandomDirection` (`local.MuzzleDirection`) (`local.Spread`))))
  (bind (_outstartposition_3 _outdirection_3) (`self.GetVectorsMuzzleOwner` (`local.OwnerLocation`) (`self.GetRandomDirection` (`local.OwnerDirection`) (`local.Spread`)) (`local.MuzzleLocation`)))
  ;[0 0 0 0.5] Shoot Origin Selector
  (switch `/Game/Blueprints/Guns/E_ShootOrigin` ShootOrigin
    (:`NewEnumerator0`
      ;[0 0 0 0.5] Use Owner Position and Direction
      (return _outstartposition _outdirection))
    (:`NewEnumerator1`
      ;[0 0 0 0.5] Use Muzzle Position and Direction
      (return _outstartposition_2 _outdirection_2))
    (:`NewEnumerator2`
      ;[0 0 0 0.5] Use Muzzle Position and Owner Direction
      (return _outstartposition_3 _outdirection_3))))

(fn `GetRandomDirection`
  (params (InitialDirection :type "Vector Structure") (Spread :type "Float (double-precision)"))
  (returns (RandomizedDirection :type "Vector Structure"))
  (return (`KismetMathLibrary.RandomUnitVectorInConeInDegrees` InitialDirection Spread)))