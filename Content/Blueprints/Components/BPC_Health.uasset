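; Health component that tracks an actor's current health and broadcasts damage, death and heal events.
; BeginPlay fills CurrentHealth from MaxHealth.
; DealDamage and Damage subtract health while it is above zero, call OnDamage and share a death check that calls OnDeath; Damage's DamageDealer input is unused.
; Heal adds health and calls OnHeal unless health equals the maximum, without clamping the result.
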(event `self.ReceiveBeginPlay`
  ;[0 0 0 0.5] Set max heath on begin
  (set `self.CurrentHealth` (`self.MaxHealth`)))

(event `self.DealDamage`
  (params (DamageDealer :type "Actor Object Reference") (DamageAmount :type "Float (single-precision)"))
  ;[0 0 0 0.5] Damage
  (if (> (`self.CurrentHealth`) 0.0)
    (set `self.CurrentHealth` (- (`self.CurrentHealth`) DamageAmount))
    (`self.OnDamage`)
    ;[0 0 0 0.5] Check if dead
    (if (<= (`self.CurrentHealth`) 0.0) :!label _label
      (`self.OnDeath`))))

(event `Damage`
  (params (DamageDealer :type "Actor Object Reference") (DamageAmount :type "Float (double-precision)"))
  ;[0 0 0 0.5] Damage
  (if (> (`self.CurrentHealth`) 0.0)
    (set `self.CurrentHealth` (- (`self.CurrentHealth`) DamageAmount))
    (`self.OnDamage`)
    (goto _label)))

(event `Heal`
  (params (HealAmount :type "Float (double-precision)"))
  ;[0 0 0 0.5] Heal
  (if (not (== (`self.CurrentHealth`) (`self.MaxHealth`)))
    (set `self.CurrentHealth` (+ (`self.CurrentHealth`) HealAmount))
    (`self.OnHeal`)))