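; Weapon equipment component that keeps an array of weapon actors and tracks which one is held.
; BeginPlay and AddWeapon check each actor for the Weapon interface, hiding valid ones and printing errors for others.
; Previous/next events wrap the index with modulo into SwitchWeapon, which stops and hides the old weapon, reveals the new one and fires OnHeldWeaponChanged.
; Attach and detach nodes are left unconnected.
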(event `Add Weapon`
  (params (Weapon :type "Actor Object Reference"))
  ;[0 0 0 0.5] Add Weapon
  (`self.EvaluateWeaponValid` Weapon)
  (`KismetArrayLibrary.Array_Add` (`self.Weapons`) Weapon))

(event `Evaluate`
  ;[0 0 0 0.5] Check if All Actors implement the Weapons interface
  (for _array_element (`self.Weapons`) :!label _label
    (`self.EvaluateWeaponValid` _array_element)))

(event `self.ReceiveBeginPlay`
  ;[0 0 0 0.5] Check if All Actors implement the Weapons interface
  (goto _label))

(event `Set Previous Weapon`
  ;[0 0 0 0.5] Set the Previous Weapon in the Array
  (`self.SwitchWeapon` (`self.LoopIndex` (- (`self.HeldWeaponIndex`) 1))))

(event `Set Next Weapon`
  ;[0 0 0 0.5] Set the Next Weapon in the Array
  (`self.SwitchWeapon` (`self.LoopIndex` (+ (`self.HeldWeaponIndex`) 1))))

(fn `CheckHasWeapons`
  (returns (HasWeapons :type Boolean))
  (return (> (`KismetArrayLibrary.Array_Length` (`self.Weapons`)) 0)))

(fn `CompareWeaponIndex`
  (params (Index :type Integer))
  (returns (Result :type Boolean))
  (return (== Index (`self.HeldWeaponIndex`))))

(fn `EvaluateIndexValid`
  (params (Index :type Integer))
  (returns (Result :type Boolean))
  ;[0 0 0 0.5] Check if index is between 0 and the length of the array - 1 (within the array)
  (return (and (>= (`local.Index`) 0) (< (`local.Index`) (`KismetArrayLibrary.Array_Length` (`self.Weapons`))))))

(fn `EvaluateWeaponValid`
  (params (Actor :type "Actor Object Reference"))
  ;[0 0 0 0.5] Check if Actor Implements the Weapons Interface
  (if (`KismetSystemLibrary.DoesImplementInterface` Actor "/Script/SparkleblastWeapons.Weapon")
    ;[0 0 0 0.5] Set Weapon Hidden
    (`Actor.SetActorHiddenInGame` Actor true)
    (else
      ;[0 0 0 0.5] Print Error
      (`KismetSystemLibrary.PrintString` (`KismetStringLibrary.Concat_StrStr` (`KismetSystemLibrary.GetObjectName` (`self.GetOwner`)) ": Actor does not implement interface Weapons!") true true (struct :`R` 1.0 :`G` 0.036976 :`A` 1.0)))))

(fn `GetHeldWeapon`
  (returns (Weapon :type "Actor Object Reference"))
  (return (`|GetArrayItem` (`self.Weapons`) (`self.HeldWeaponIndex`))))

(fn `LoopIndex`
  (params (Index :type Integer))
  (returns (Result :type Integer))
  (bind _returnvalue (`KismetArrayLibrary.Array_Length` (`self.Weapons`)))
  (return (mod (+ (`local.Index`) _returnvalue) (`KismetMathLibrary.Max` _returnvalue 1))))

(fn `SwitchWeapon`
  (params (index :type Integer))
  ;[0 0 0 0.5] Switch Weapon (Ignores if No Weapons or Index is Not Valid)
  (if (`self.CheckHasWeapons`)
    (if (`self.EvaluateIndexValid` (`local.index`))
      (if (not (`self.CompareWeaponIndex` (`local.index`)))
        (set `self.HeldWeaponIndex` (`local.index`))
        (`self.UpdateHeldWeapon`)))))

(fn `UpdateHeldWeapon`
  (bind _output (`|GetArrayItem` (`self.Weapons`) (`self.HeldWeaponIndex`)))
  ;[0 0 0 0.5] Stop if No Weapons
  (if (`self.CheckHasWeapons`)
    ;[0 0 0 0.5] Set Current Held Weapon Hidden, Unattach from Component and disable shooting if shooting
    (`|ExecutionSequence`
      (:`then_0`
        (bind _heldweapon (`self.HeldWeapon`)
          (:`then`
            (if (!= _heldweapon (`|GetArrayItem` (`self.Weapons`) (`self.HeldWeaponIndex`)))
              (message `Weapon.StopAttacking` (`self.HeldWeapon`))
              (`Actor.SetActorHiddenInGame` (`self.HeldWeapon`) true)))
          (:`else`)))
      (:`then_1`
        ;[0 0 0 0.5] Attach to Component and Unhide New Held Weapon
        (if (`KismetSystemLibrary.IsValid` _output)
          (set `self.HeldWeapon` _output)
          (`|ExecutionSequence`
            (:`then_0`
              (`Actor.SetActorHiddenInGame` (`self.HeldWeapon`) false)
              (`self.OnHeldWeaponChanged` (`self.HeldWeapon`)))
            (:`then_1`
              (`KismetSystemLibrary.PrintString` (`KismetStringLibrary.Concat_StrStr` "Held Weapon: " (`KismetSystemLibrary.GetDisplayName` (`self.HeldWeapon`)))))))))))