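; Explosion component that applies distance-based knockback and damage to BP_Target actors in a radius, with FMOD sound, camera shake and optional debug sphere.
; A line trace finds each target's impact point, falling back to actor location, to drive force and damage curves.
; The player uses LaunchCharacter while others get movement velocity set, with axis and shooter-push options.
; Damage goes through BPC_Health, sparing the shooter, and CallOnExplode fires afterwards.
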(event `Explode`
  (params (Shooter :type "Object Object Reference") (ExplosionLocations :type "Vector Structure"))
  ;[0 0 0 0.5] Find Targets
  (set `self.ExplosionOwner` Shooter)
  (bind _output_get (set `self.ExplosionLocation` ExplosionLocations))
  (bind (_outactors _returnvalue) (`KismetSystemLibrary.SphereOverlapActors` _output_get (`self.Radius`) (`|MakeArray` "ObjectTypeQuery1" "ObjectTypeQuery2" "ObjectTypeQuery3" "ObjectTypeQuery4" :!type "EObjectTypeQuery Enum") "/Game/Blueprints/BP_Target.BP_Target_C"))
  (`|ExecutionSequence`
    (:`then_0`
      ;[0 0 0 0.5] Loop Through All Overlapping Actors
      (if _returnvalue
        (for _array_element _outactors
          (`self.ExplodeOnTarget` _array_element))))
    (:`then_1`
      ;[0 0 0 0.5] Debug Draw Sphere
      (if (`self.ShowDebugSphere`)
        (`KismetSystemLibrary.DrawDebugSphere` (`self.ExplosionLocation`) (`self.Radius`) 12 (struct :`R` 1.0 :`A` 1.0) (`self.DebugSphereDuration`) 1.0)))
    (:`then_2`
      ;[0 0 0 0.5] Play Sound
      (`/Game/Blueprints/FL_FMODFunctions.PlayOneShotAtLocation` (`self.ExplosionFMODEvent`) (`self.ExplosionLocation`)))
    (:`then_3`
      ;[0 0 0 0.5] Camera Shake
      (`GameplayStatics.PlayWorldCameraShake` (`self.ShakeEffect`) (`self.ExplosionLocation`) 0.0 (`self.ShakeRadius`) (`self.ShakeFalloff`)))
    (:`then_4`
      ;[0 0 0 0.5] Explosion Callback
      (`self.OnExplode` (`self.ExplosionLocation`)))))

(fn `CalcDistanceAndDirection`
  (params (HitLocation :type "Vector Structure"))
  (returns (Distance :type "Float (double-precision)") (Direction :type "Vector Structure"))
  (return (`KismetMathLibrary.Vector_Distance` HitLocation (`self.ExplosionLocation`)) (`KismetMathLibrary.Normal` (- HitLocation (`self.ExplosionLocation`)))))

(fn `ExplodeOnTarget`
  (params (HitTarget :type "Actor Object Reference"))
  (locals (HitTargetLocation :type "Vector Structure") (Distance :type "Float (double-precision)") (FractionDecimal :type "Float (double-precision)") (TargetHit :type Boolean) (Direction :type "Vector Structure") (LaunchDirection :type "Vector Structure") (VerticalLaunch :type "Float (double-precision)"))
  (bind _returnvalue (`GameplayStatics.GetPlayerCharacter` 0))
  (bind _pushshooter (`self.PushShooter`))
  (bind (_direction_x _direction_y _direction_z) (`KismetMathLibrary.BreakVector` (`local.Direction`)))
  (bind (_direction_x_2 _direction_y_2) (`KismetMathLibrary.BreakVector` (`local.Direction`)))
  (bind (_launchdirection_x _launchdirection_y) (`KismetMathLibrary.BreakVector` (`local.LaunchDirection`)))
  (bind _returnvalue_2 (`Actor.GetComponentByClass` (`local.HitTarget`) "/Game/Blueprints/Components/BPC_Health.BPC_Health_C"))
  (bind _returnvalue_3 (`Actor.GetComponentByClass` (`local.HitTarget`) "/Script/Engine.MovementComponent"))
  (bind (_distance _direction) (`self.CalcDistanceAndDirection` (`local.HitTargetLocation`)))
  (bind _returnvalue_4 (* (`CurveFloat.GetFloatValue` (`self.ForceByDistance`) (`local.FractionDecimal`)) (`KismetMathLibrary.Normal` (`local.LaunchDirection`))))
  (bind _returnvalue_5 (+ (`self.AdditionalDamage`) (`CurveFloat.GetFloatValue` (`self.DamageByDistance`) (`local.FractionDecimal`))))
  ;[0 0 0 0.5] Get Impact Point of Actor
  (set `local.HitTargetLocation` (`Actor.K2_GetActorLocation` (`local.HitTarget`)))
  (bind (_outhits _returnvalue_6) (`KismetSystemLibrary.LineTraceMulti` (`self.ExplosionLocation`) (`local.HitTargetLocation`) "TraceTypeQuery3"))
  (if _returnvalue_6
    (for _array_element _outhits
      (bind (_bblockinghit _binitialoverlap _time _distance_2 _location _impactpoint _normal _impactnormal _physmat _hitactor) (`GameplayStatics.BreakHitResult` _array_element))
      ;[0 0 0 0.5] Found Actor. Set Distance and Direction
      (if (== _hitactor (`local.HitTarget`))
        (set `local.TargetHit` true)
        (bind (_distance_3 _direction_2) (`self.CalcDistanceAndDirection` _impactpoint))
        (set `local.Distance` _distance_3)
        (set `local.Direction` _direction_2)
        (break)))
    (if (not (`local.TargetHit`))
      ;[0 0 0 0.5] Actor not found. Set Distance and Direction
      (set `local.Distance` _distance :!label _label)
      (set `local.Direction` _direction))
    (else
      (goto _label)))
  ;[0 0 0 0.5] Set Fraction Decimal
  (set `local.FractionDecimal` (/ (`local.Distance`) (`self.Radius`)))
  (`|ExecutionSequence`
    (:`then_0`
      ;[0 0 0 0.5] Start Add Force
      (if (or (and (!= (`self.ExplosionOwner`) (`local.HitTarget`)) (not _pushshooter)) _pushshooter)
        ;[0 0 0 0.5] Setting Launch Direction
        (`|ExecutionSequence`
          (:`then_0`
            (if (`self.ApplyHorizontalForce`)
              (set `local.LaunchDirection` (`KismetMathLibrary.MakeVector` _direction_x_2 _direction_y_2))))
          (:`then_1`
            (if (`self.ApplyVerticalForce`)
              (set `local.VerticalLaunch` _direction_z)
              ;[0 0 0 0.5] Keep Vertical Launch positive if Ignore Downwards Force True
              (`|ExecutionSequence`
                (:`then_0`
                  (if (`self.IgnoreDownwardsForce`)
                    (set `local.VerticalLaunch` (`KismetMathLibrary.FMax` 0.0 (`local.VerticalLaunch`)))))
                (:`then_1`
                  (set `local.LaunchDirection` (`KismetMathLibrary.MakeVector` _launchdirection_x _launchdirection_y (`local.VerticalLaunch`)))))))
          (:`then_2`
            ;[0 0 0 0.5] If Player, Launch Player
            (if (!= (`local.HitTarget`) _returnvalue)
              ;[0 0 0 0.5] If has Movement Component, Set Velocity for launching
              (`/Engine/EditorBlueprintResources/StandardMacros.IsValid` _returnvalue_3
                (:`Is Valid`
                  (set `MovementComponent.Velocity` (* _returnvalue_4 (`self.MultiplierLaunchNonPlayer`)) _returnvalue_3)))
              (else
                (`Character.LaunchCharacter` _returnvalue _returnvalue_4 false true)))))))
    (:`then_1`
      ;[0 0 0 0.5] Deal Damage
      (if (!= (`self.ExplosionOwner`) (`local.HitTarget`))
        (if (`KismetSystemLibrary.IsValid` _returnvalue_2)
          (`/Game/Blueprints/Components/BPC_Health.Damage` _returnvalue_2 (`self.GetOwner`) _returnvalue_5)
          (`KismetSystemLibrary.PrintString` (`KismetStringLibrary.Concat_StrStr` "Explosion Damage:" (`KismetStringLibrary.Conv_DoubleToString` _returnvalue_5))))))))