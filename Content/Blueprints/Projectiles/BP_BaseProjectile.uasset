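; Base projectile Blueprint that takes damage, speed, piercing and shooter, scales its movement velocity, and reports what it overlaps.
; OnOverlap ignores other projectiles and calls separate dispatchers for the shooter, targets with BPC_Health, and non-targets unless IgnoreEnvironment is set.
; Overlap events feed that check, and a manual sphere check one tick after BeginPlay catches actors overlapping at spawn, stopping at the first accepted hit.
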(event `self.Constructor`
  (params (AttackDamage :type "Float (single-precision)") (Speed :type "Float (single-precision)") (Piercing :type Boolean) (Shooter :type "Actor Object Reference"))
  ;[0 0 0 0.5] Constructor
  (set `self.Damage` AttackDamage)
  (set `MovementComponent.Velocity` (* (`MovementComponent.Velocity` (`self.ProjectileMovement`)) Speed) (`self.ProjectileMovement`))
  (set `self.Piercing` Piercing)
  (set `self.Shooter` Shooter))

(event `self.ReceiveBeginPlay`
  ;[0 0 0 0.5] Check for Overlaps when Spawned
  (`KismetSystemLibrary.DelayUntilNextTick`)
  (`self.ManualCheckOverlap`))

(event `self.ReceiveActorBeginOverlap`
  (params (OtherActor :type "Actor Object Reference"))
  ;[0 0 0 0.5] Overlap
  (`self.OnOverlap` OtherActor))

(fn `ManualCheckOverlap`
  (locals (OverlappingActors :type "Array of Actor Object Reference"))
  ;[0 0 0 0.5] Checks whether there are any actors overlapping with the projectile
  (bind _output_get (set `local.OverlappingActors` (`PrimitiveComponent.GetOverlappingActors` (`self.Sphere`) null)))
  (for _array_element _output_get
    (bind _hashit (`self.OnOverlap` _array_element))
    (if _hashit
      (break))))

(fn `OnOverlap`
  (params (OtherActor :type "Actor Object Reference"))
  (returns (HasHit :type Boolean))
  ;[0 0 0 0.5] On Overlap
  (if (`KismetSystemLibrary.IsValid` (`local.OtherActor`))
    (if (not (`KismetSystemLibrary.DoesImplementInterface` (`local.OtherActor`) "/Script/SparkleblastWeapons.Projectile"))
      (bind _shooter (`self.Shooter`)
        (:`then`
          (if (!= _shooter (`local.OtherActor`))
            (if (`KismetSystemLibrary.IsValid` (`self.GetComponentByClass` (`local.OtherActor`) "/Game/Blueprints/Components/BPC_Health.BPC_Health_C"))
              (`self.OnHitTarget` (`self.Damage`) (`local.OtherActor`))
              (return true)
              (elif (not (`self.IgnoreEnvironment`))
                (`self.OnHitNonTarget` (`self.Damage`) (`local.OtherActor`))
                (return true)))
            (else
              (`self.OnHitShooter`)
              (return false))))
        (:`else`
          (return false)))
      (else
        (return false)))
    (else
      (return false))))

(fn `UserConstructionScript`)