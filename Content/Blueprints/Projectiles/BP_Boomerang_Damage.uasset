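; Boomerang damage projectile that hurts targets through their health component, destroying itself on hit unless piercing.
; After a return delay, or on hitting a non-target, it ignores the environment and homes back to its shooter via the projectile movement component.
; While returning, Tick boosts homing acceleration once near the shooter and destroys the projectile when close enough; hitting the shooter also destroys it.
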(event `self.ReceiveBeginPlay`
  (`|ExecutionSequence`
    (:`then_0`
      ;[0 0 0 0.5] On Hit Target
      (add `self.OnHitTarget` (delegate `On Hit Target`))
      ;[0 0 0 0.5] On Hit Non Target
      (add `self.OnHitNonTarget` (delegate `On Hit Non Target`))
      ;[0 0 0 0.5] Check for Overlaps
      (`parent.ReceiveBeginPlay`))
    (:`then_1`
      ;[0 0 0 0.5] Homing Logic
      (`KismetSystemLibrary.Delay` (`self.ReturnDelay`))
      (set `self.IgnoreEnvironment` true :!label _label)
      (set `ProjectileMovementComponent.HomingTargetComponent` (`Actor.RootComponent` (`self.Shooter`)) (`self.ProjectileMovement`))
      (set `ProjectileMovementComponent.bIsHomingProjectile` true (`self.ProjectileMovement`))
      (add `self.OnHitShooter` (delegate `DestroySelf`))
      (set `self.Returning` true))))

(event `On Hit Target` :!signature `self.OnHitTarget`
  (params (Damage :type "Float (double-precision)") (HitActor :type "Actor Object Reference"))
  ;[0 0 0 0.5] On Hit Target
  (`/Game/Blueprints/Components/BPC_Health.Damage` (`self.GetComponentByClass` HitActor "/Game/Blueprints/Components/BPC_Health.BPC_Health_C") self Damage)
  ;[0 0 0 0.5] Check if Projectile is Piercing
  (if (not (`self.Piercing`))
    (`self.K2_DestroyActor`)))

(event `On Hit Non Target` :!signature `self.OnHitNonTarget`
  (params (Damage :type "Float (double-precision)") (HitActor :type "Actor Object Reference"))
  ;[0 0 0 0.5] On Hit Non Target
  (`self.ReturnToShooter`))

(event `self.ReceiveTick`
  (params (DeltaSeconds :type "Float (single-precision)"))
  ;[0 0 0 0.5] Speed Up Returning When Close to Shooter
  (if (`self.Returning`)
    (`|ExecutionSequence`
      (:`then_0`
        (if (not (`self.HasSpedUp`))
          (if (<= (`self.GetDistanceFromShooter`) (`self.SpedUpDistance`))
            (set `ProjectileMovementComponent.HomingAccelerationMagnitude` (`self.SpedUpAcceleration`) (`self.ProjectileMovement`))
            (set `self.HasSpedUp` true))))
      (:`then_1`
        ;[0 0 0 0.5] Destroy Self When Close to Shooter
        (if (<= (`self.GetDistanceFromShooter`) (`self.ReturnDistance`))
          (`self.DestroySelf`))))))

(event `ReturnToShooter`
  ;[0 0 0 0.5] Homing Logic
  (set `MovementComponent.Velocity` (0.0 0.0 0.0) (`self.ProjectileMovement`))
  (goto _label))

(event `DestroySelf`
  ;[0 0 0 0.5] Homing Logic
  (`self.K2_DestroyActor`))

(fn `GetDistanceFromShooter`
  (returns (Distance :type "Float (double-precision)"))
  (return (`KismetMathLibrary.Vector_Distance` (`self.K2_GetActorLocation`) (`self.K2_GetActorLocation` (`self.Shooter`)))))

(fn `UserConstructionScript`
  (`parent.UserConstructionScript`))