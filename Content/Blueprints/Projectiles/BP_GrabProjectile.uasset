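; Grapple projectile for an offhand ability that pulls the target it hits to a point in front of the shooter.
; On hit it snaps to the target's surface via trace, attaches, adds a pull component, starts a time-limit timer and stuns via BPI_EnemyStun.
; Tick updates the pull destination from shooter aim and both actors' bounds, or range-checks before impact.
; DestroySelf ends the pull and notifies the offhand, including on misses or over-range.
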(event `CheckDistanceFromShooter`
  ;[0 0 0 0.5] Distance Limit
  (if (> (`KismetMathLibrary.Vector_Distance` (`self.K2_GetActorLocation`) (`self.StartPosition`)) (`self.ProjectileMaxDistance`))
    (`KismetSystemLibrary.PrintString` "GrappleProjectile too far, deleting self")
    (`self.DestroySelf`)))

(event `GrabConstructor`
  (params (PullDelay :type "Float (double-precision)") (PullTimeLimit :type "Float (double-precision)") (PullSpeed :type "Float (double-precision)") (DistanceEndPosition :type "Float (double-precision)") (StunDurationAfter :type "Float (double-precision)") (ProjectileMaxDistance :type "Float (double-precision)") (ConnectedOffhand :type "/Game/Blueprints/Offhand/BP_BaseOffhand Object Reference"))
  ;[1 0 0 0.5] Temporary Constructor until I figure out something else
  (set `self.PullDelay` PullDelay)
  (set `self.PullTimeLimit` PullTimeLimit)
  (set `self.PullSpeed` PullSpeed)
  (set `self.DistanceEndPosition` DistanceEndPosition)
  (set `self.StunDurationAfter` StunDurationAfter)
  (set `self.ProjectileMaxDistance` ProjectileMaxDistance)
  (set `self.ConnectedOffhand` ConnectedOffhand))

(event `Pull Update`
  (bind _shooterlook (`self.ShooterLook`))
  ;[0 0 0 0.5] Pull Update
  (`self.PullComponent`
    (:`then`
      (set `/Game/Blueprints/Components/BPC_Pull.Destination` (+ (`SceneComponent.K2_GetComponentLocation` _shooterlook) (* (`SceneComponent.GetForwardVector` _shooterlook) (+ (`KismetMathLibrary.FMax` (.x (`.BoxExtent` (`self.GetActorBounds` (`self.HitTarget`) true false))) (.y (`.BoxExtent` (`self.GetActorBounds` (`self.HitTarget`) true false)))) (`self.DistanceEndPosition`) (`KismetMathLibrary.FMax` (.x (`.BoxExtent` (`self.GetActorBounds` (`self.Shooter`) true false))) (.y (`.BoxExtent` (`self.GetActorBounds` (`self.Shooter`) true false))))))) (`self.PullComponent`)))
    (:`else`
      (`self.DestroySelf`))))

(event `self.ReceiveBeginPlay`
  (set `self.StartPosition` (`self.K2_GetActorLocation`))
  (add `self.OnHitTarget` (`|CreateDelegate` :!event `On Hit Target`))
  ;[0 0 0 0.5] On hit non target
  (add `self.OnHitNonTarget` (delegate `On Hit Non Target`))
  ;[0 0 0 0.5] Check for overlaps
  (`parent.ReceiveBeginPlay`))

(event `Unbind Events`
  (remove `self.OnHitTarget` (`|CreateDelegate` :!event `On Hit Target`))
  ;[0 0 0 0.5] On hit non target
  (remove `self.OnHitNonTarget` (delegate `On Hit Non Target`)))

(event `self.ReceiveTick`
  (params (DeltaSeconds :type "Float (single-precision)"))
  ;[0 0 0 0.5] Tick
  (if (`self.PullingActive`)
    (`self.Pull Update`)
    (else
      (`self.CheckDistanceFromShooter`))))

(event `On Hit Non Target` :!signature `self.OnHitNonTarget`
  (params (Damage :type "Float (double-precision)") (HitActor :type "Actor Object Reference"))
  ;[0 0 0 0.5] On hit non target
  (`KismetSystemLibrary.PrintString` "Hit Non Target")
  (`self.DestroySelf`))

(event `DestroySelf`
  ;[0 0 0 0.5] Destroy Self
  (`KismetSystemLibrary.K2_ClearAndInvalidateTimerHandle` (`self.PullTimer`))
  (set `/Game/Blueprints/Offhand/BP_BaseOffhand.AbilityActive` false (`self.ConnectedOffhand`))
  (`/Game/Blueprints/Offhand/BP_BaseOffhand.OnAbilityFinished` (`self.ConnectedOffhand`))
  (`|ExecutionSequence`
    (:`then_0`
      (bind _pullcomponent (`self.PullComponent`)
        (:`then`
          (`/Game/Blueprints/Components/BPC_Pull.DestroyPull` _pullcomponent))
        (:`else`)))
    (:`then_1`
      (`self.K2_DestroyActor`))))

(event `On Hit Target` :!signature `self.OnHitTarget`
  (params (Damage :type "Float (double-precision)") (HitActor :type "Actor Object Reference"))
  ;[0 0 0 0.5] On hit target
  (`KismetSystemLibrary.PrintString` "Hit Target")
  (`self.Unbind Events`)
  (set `MovementComponent.Velocity` (0.0 0.0 0.0) (`self.ProjectileMovement`))
  (`self.SetLifeSpan` 0.0)
  (set `self.HitTarget` HitActor)
  (`|ExecutionSequence`
    (:`then_0`
      (`self.SetPositionCenterClose`))
    (:`then_1`
      (bind _returnvalue (`AddComponent|NODE_AddBPC_Pull-0` :`self` (`self.HitTarget`)))
      (bind _output_get (set `self.PullComponent` _returnvalue))
      (`/Game/Blueprints/Components/BPC_Pull.Constructor` _output_get (`self.K2_GetActorLocation` (`self.Shooter`)) (`self.PullSpeed`) (`self.PullDelay`))
      (`/Game/Blueprints/Components/BPC_Pull.StartPulling` _output_get)
      (`self.K2_AttachToActor` (`self.HitTarget`) "None" "KeepWorld" "KeepWorld" "KeepWorld")
      (set `self.PullingActive` true)
      (remove `/Game/Blueprints/Offhand/BP_BaseOffhand.OnSwapped` (`self.ConnectedOffhand`) (`|CreateDelegate` :!event `DestroySelf`))
      (bind _returnvalue_2 (`KismetSystemLibrary.K2_SetTimerDelegate` (`|CreateDelegate` :!event `DestroySelf`) (`self.PullTimeLimit`)))
      (set `self.PullTimer` _returnvalue_2)
      (if (`KismetSystemLibrary.DoesImplementInterface` (`self.HitTarget`) "/Game/Blueprints/NPC/Enemies/BPI_EnemyStun.BPI_EnemyStun_C")
        (message `/Game/Blueprints/NPC/Enemies/BPI_EnemyStun.Stun` (`self.HitTarget`) (+ 0.25 (`self.PullTimeLimit`)))))))

(fn `SetPositionCenterClose`
  (bind _outhits (`KismetSystemLibrary.LineTraceMulti` (`self.K2_GetActorLocation` (`self.Shooter`)) (`self.K2_GetActorLocation` (`self.HitTarget`)) "TraceTypeQuery3"))
  (for _array_element _outhits
    (bind (_bblockinghit _binitialoverlap _time _distance _location _impactpoint _normal _impactnormal _physmat _hitactor) (`GameplayStatics.BreakHitResult` _array_element))
    (if (== _hitactor (`self.HitTarget`))
      (`self.K2_SetActorLocation` _location false true))))

(fn `UserConstructionScript`
  (`parent.UserConstructionScript`))