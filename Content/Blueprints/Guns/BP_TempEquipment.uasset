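; BP_TempEquipment is a Blueprint that exercises the BPCEquipment component, apparently as a temporary test for weapon switching and firing.
; On BeginPlay it updates the held weapon and sends it StartAttackingMessage, passing the weapon itself as OwnerShooter.
; After a short delay it switches to the next weapon and starts that one attacking the same way.
; No stop-attack call is made in its graph.
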(event `self.ReceiveBeginPlay`
  (bind _weapon (`/Game/Blueprints/Components/BPC_Equipment.GetHeldWeapon` (`self.BPC_Equipment`)))
  (bind _weapon_2 (`/Game/Blueprints/Components/BPC_Equipment.GetHeldWeapon` (`self.BPC_Equipment`)))
  (`/Game/Blueprints/Components/BPC_Equipment.UpdateHeldWeapon` (`self.BPC_Equipment`))
  (message `Weapon.StartAttacking` _weapon_2 null _weapon_2)
  (`KismetSystemLibrary.Delay` 3.0)
  (`/Game/Blueprints/Components/BPC_Equipment.Set Next Weapon` (`self.BPC_Equipment`))
  (message `Weapon.StartAttacking` _weapon null _weapon))

(fn `UserConstructionScript`)