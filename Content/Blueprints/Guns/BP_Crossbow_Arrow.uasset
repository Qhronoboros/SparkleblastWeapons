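; BP_Crossbow_Arrow is a crossbow projectile that explodes on impact, whether or not it hits a target.
; It binds the hit-target and hit-non-target events before calling parent BeginPlay, which checks for overlaps.
; A target hit first applies damage through the actor's BPC_Health component.
; Both hit paths then trigger BPCExplode at the arrow's location, credited to the shooter, and destroy the arrow.
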(event `self.ReceiveBeginPlay`
  ;[0 0 0 0.5] On Hit Target
  (add `self.OnHitTarget` (delegate `On Hit Target`))
  ;[0 0 0 0.5] On Hit Non Target
  (add `self.OnHitNonTarget` (delegate `On Hit Non Target`))
  ;[0 0 0 0.5] Check for Overlaps
  (`parent.ReceiveBeginPlay`))

(event `On Hit Target` :!signature `self.OnHitTarget`
  (params (Damage :type "Float (double-precision)") (HitActor :type "Actor Object Reference"))
  ;[0 0 0 0.5] On Hit Target
  (`/Game/Blueprints/Components/BPC_Health.Damage` (`self.GetComponentByClass` HitActor "/Game/Blueprints/Components/BPC_Health.BPC_Health_C") self Damage)
  ;[0 0 0 0.5] On Hit Non Target
  (`/Game/Blueprints/Components/BPC_Explode.Explode` (`self.BPC_Explode`) (`self.Shooter`) (`self.K2_GetActorLocation`) :!label _label)
  (`self.K2_DestroyActor`))

(event `On Hit Non Target` :!signature `self.OnHitNonTarget`
  (params (Damage :type "Float (double-precision)") (HitActor :type "Actor Object Reference"))
  ;[0 0 0 0.5] On Hit Non Target
  (goto _label))

(fn `UserConstructionScript`
  (`parent.UserConstructionScript`))