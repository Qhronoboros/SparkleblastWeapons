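; Base gun Blueprint that handles firing feedback: FMOD audio, camera shake and player recoil pushback.
; InitializeWeapon fills the blackboard with muzzle, shooter and head, then binds the fired callback, which shakes and pushes only if CameraShake is valid.
; ApplyFirePushback launches only the player opposite head facing, scaling horizontal force by a movement-versus-look angle curve, blending with existing velocity and keeping the higher vertical speed.
; Mouse input test is unused.
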(event `self.InitializeWeapon`
  (params (Shooter :type "Actor Object Reference") (Head :type "SceneComponent Object Reference"))
  ;[0 0 0 0.5] Initialize Weapon
  (`|ExecutionSequence`
    (:`then_0`
      (`self.SetupBlackboard` (`self.BlackboardComponent`) (`self.Muzzle`) Shooter Head)
      (add `self.OnGunFired` (delegate `OnGunFiredCallback`)))))

(event `self.ReceiveBeginPlay`
  ;[0 0 0 0.5] Initialize Weapon
)

(event `OnGunFiredCallback` :!signature `self.OnGunFired`
  (params (Vec1 :type "Vector Structure") (Vec2 :type "Vector Structure"))
  ;[0 0 0 0.5] On Gun Fired Callback
  ;;[0 0 0 0.5] Play Gun Fire Audio
  (`/Game/Blueprints/FL_FMODFunctions.PlayOneShot2D` (`self.ShootFMODEvent`))
  ;;[0 0 0 0.5] Camera Shake
  (bind _camerashake (`self.CameraShake`)
    (:`then`
      (`GameplayStatics.PlayWorldCameraShake` _camerashake (`self.K2_GetActorLocation`) 0.0 100.0 0.0)
      ;;[0 0 0 0.5] Apply Fire Pushback
      (bind _asscene_component (cast `SceneComponent` (`BlackboardComponent.GetValueAsObject` (`self.BlackboardComponent`) (`self.HeadKey`))))
      (bind _asactor (cast `Actor` (`BlackboardComponent.GetValueAsObject` (`self.BlackboardComponent`) (`self.ShooterKey`))))
      (`self.ApplyFirePushback` _asactor _asscene_component))
    (:`else`)))

(event `self.ReceiveTick`
  (params (DeltaSeconds :type "Float (single-precision)"))
  ;[1 0 0 0.5] Player Input Test (Not Getting Used)
)

(fn `ApplyFirePushback`
  (params (Shooter :type "Actor Object Reference") (Head :type "SceneComponent Object Reference"))
  (locals (OwnerBackwardVector :type "Vector Structure") (PlayerCharacter :type "Character Object Reference") (PlayerVelocity :type "Vector Structure") (HorizontalPushbackVelocity :type "Vector Structure") (PlayerHorizontalMagnitude :type "Float (double-precision)") (HorizontalPushbackMagnitude :type "Float (double-precision)") (HorizontalLaunchVelocity :type "Vector Structure") (AngleMoveVelocityAndLookDirection :type "Float (double-precision)") (Pushback2D :type "Vector Structure") (VerticalPushback :type "Float (double-precision)") (PlayerMovement2D :type "Vector Structure") (PlayerInputVector :type "Vector Structure"))
  (bind _returnvalue (`GameplayStatics.GetPlayerCharacter` 0))
  (bind (_playervelocity_x _playervelocity_y) (`KismetMathLibrary.BreakVector` (`local.PlayerVelocity`)))
  (bind (_playervelocity_x_2 _playervelocity_y_2 _playervelocity_z) (`KismetMathLibrary.BreakVector` (`local.PlayerVelocity`)))
  (bind (_ownerbackwardvector_x _ownerbackwardvector_y) (`KismetMathLibrary.BreakVector` (`local.OwnerBackwardVector`)))
  (bind (_returnvalue_x _returnvalue_y _returnvalue_z) (`KismetMathLibrary.BreakVector` (* (`self.PushbackForce`) (`KismetMathLibrary.Normal` (`KismetMathLibrary.MakeVector` _ownerbackwardvector_x _ownerbackwardvector_y (`local.VerticalPushback`))))))
  ;[0 0 0 0.5] Fire Pushback (Only works for Player)
  (if (== (`local.Shooter`) _returnvalue)
    (bind _output_get (set `local.PlayerCharacter` _returnvalue))
    (set `local.PlayerInputVector` (`KismetMathLibrary.Normal` (`Pawn.GetLastMovementInputVector` _output_get)))
    (bind _charactermovement (`Character.CharacterMovement` (`local.PlayerCharacter`))
      (:`then`
        (bind _output_get_2 (set `local.PlayerVelocity` (`MovementComponent.Velocity` _charactermovement)))
        (set `local.PlayerHorizontalMagnitude` (`KismetMathLibrary.VSize2D` (`KismetMathLibrary.Conv_VectorToVector2D` _output_get_2)))
        (bind _output_get_3 (set `local.OwnerBackwardVector` (* (`SceneComponent.GetForwardVector` (`local.Head`)) -1)))
        (set `local.VerticalPushback` (* (`self.VerticalPushbackAmplifier`) (.z _output_get_3)))
        (`|ExecutionSequence`
          (:`then_0`
            ;[0 0 0 0.5] Keep Vertical Pushback positive if Ignore Downwards Pushback is True
            (if (`self.IgnoreDownwardsPushback`)
              (set `local.VerticalPushback` (`KismetMathLibrary.FMax` 0.0 (`local.VerticalPushback`)))))
          (:`then_1`
            ;[0 0 0 0.5] Pushback Vector Calculations
            (if (> (`self.PushbackForce`) 0.0)
              (set `local.Pushback2D` (`KismetMathLibrary.MakeVector` _returnvalue_x _returnvalue_y))
              (set `local.VerticalPushback` _returnvalue_z)
              (set `local.PlayerMovement2D` (`KismetMathLibrary.MakeVector` _playervelocity_x _playervelocity_y))
              (set `local.AngleMoveVelocityAndLookDirection` (`KismetMathLibrary.Dot_VectorVector` (`KismetMathLibrary.Normal` (* (`local.Pushback2D`) -1.0)) (`KismetMathLibrary.Normal` (`local.PlayerInputVector`))))
              (bind _output_get_4 (set `local.HorizontalPushbackVelocity` (* (* (`KismetMathLibrary.FMax` (* (`self.HorizontalPushbackMultiplierWhenMove`) (`KismetMathLibrary.Conv_BoolToInt` (> (`local.PlayerHorizontalMagnitude`) 0.0))) 1.0) (`local.Pushback2D`)) (`CurveFloat.GetFloatValue` (`self.HorizontalPushbackMultiplierAngleCurve`) (`local.AngleMoveVelocityAndLookDirection`)))))
              (set `local.HorizontalPushbackMagnitude` (`KismetMathLibrary.VSizeXY` _output_get_4))
              (if (`self.PushbackHorizontalVelocityOverride`)
                (set `local.HorizontalLaunchVelocity` (`KismetMathLibrary.VLerp` (`local.PlayerMovement2D`) (`local.HorizontalPushbackVelocity`) (`self.PushbackHorizontalOverride`)))
                (else
                  (set `local.HorizontalLaunchVelocity` (+ (`local.PlayerMovement2D`) (`local.HorizontalPushbackVelocity`)))))
              (`|ExecutionSequence`
                (:`then_1`
                  ;[0 0 0 0.5] Apply Pushback
                  (`Character.LaunchCharacter` (`local.PlayerCharacter`) (+ (`local.HorizontalLaunchVelocity`) (`KismetMathLibrary.MakeVector` 0.0 0.0 (`KismetMathLibrary.FMax` _playervelocity_z (* (`local.VerticalPushback`) (`self.AdditionalVerticalPushbackMultiplier`))))) true (`self.PushbackVerticalVelocityOverride`))))))))
      (:`else`))))

(fn `UserConstructionScript`)