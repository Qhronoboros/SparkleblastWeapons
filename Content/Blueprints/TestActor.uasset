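; TestActor is a test Blueprint that drives an attack from the left mouse button.
; BeginPlay passes BlackboardComponent to SetupBlackboard.
; Tick polls player controller 0 for the button, calling StartAttacking on press and StopAttacking on release, rather than binding input events.
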(event `self.ReceiveBeginPlay`
  (`self.SetupBlackboard` (`self.BlackboardComponent`)))

(event `self.ReceiveTick`
  (params (DeltaSeconds :type "Float (single-precision)"))
  (bind _returnvalue (`GameplayStatics.GetPlayerController` 0))
  (`|ExecutionSequence`
    (:`then_0`
      (if (`PlayerController.WasInputKeyJustPressed` _returnvalue "LeftMouseButton")
        (`self.StartAttacking` null)))
    (:`then_1`
      (if (`PlayerController.WasInputKeyJustReleased` _returnvalue "LeftMouseButton")
        (`self.StopAttacking`)))))

(fn `UserConstructionScript`)